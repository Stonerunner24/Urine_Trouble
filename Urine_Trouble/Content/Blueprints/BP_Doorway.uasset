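; BP_Doorway is an interactable doorway that receives the door carried by BP_Renaldo and displays the matching door component.
; Interact copies Renaldo's Door into DoorAttribute, clears his slot, refreshes visibility and prints each door color's FlowDirection.
; SetVisibility, also run at construction, hides all four door components, then shows the one matching DoorType, falling back to the base Door.
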(fn `Interact`
  (params (Interactor :type "Actor Object Reference"))
  (returns (Success :type Boolean))
  (bind _asbp_renaldo (cast `/Game/Blueprints/BP_Renaldo` Interactor))
  (bind _output_get (set `self.DoorAttribute` (`/Game/Blueprints/BP_Renaldo.Door` _asbp_renaldo)))
  (set `/Game/Blueprints/BP_Renaldo.Door` (struct) _asbp_renaldo)
  (`self.Set Visibility` _output_get)
  (for _array_element (`.DoorColors_11_41CB34CC4E5D6891EB641C9B6EF046C7` (break `/Game/Blueprints/StructDoor_BP` _output_get))
    (`KismetSystemLibrary.PrintString` (`.FlowDirection_5_1F0680EF4FCEDD23878E94BE85945D01` (break `/Game/Blueprints/S_MoleculeSpec` _array_element))))
  (return true))

(fn `Set Highlight`
  (params (Active :type Boolean))
  (`parent.Set Highlight` Active))

(fn `Set Visibility`
  (params (DoorAttribute :type "/Game/Blueprints/StructDoor_BP Structure"))
  (`SceneComponent.SetVisibility` (`self.Door2`) false false)
  (`SceneComponent.SetVisibility` (`self.Door1`) false false)
  (`SceneComponent.SetVisibility` (`self.Door3`) false false)
  (`SceneComponent.SetVisibility` (`self.Door`) false false)
  (switch `int` (`.DoorType_2_A718E4EE49CCCD5E96DEC8BADD86EF52` (break `/Game/Blueprints/StructDoor_BP` DoorAttribute))
    (:`Default`
      (`SceneComponent.SetVisibility` (`self.Door`) true false :!label _label))
    (:`0`
      (goto _label))
    (:`1`
      (`SceneComponent.SetVisibility` (`self.Door1`) true false))
    (:`2`
      (`SceneComponent.SetVisibility` (`self.Door2`) true false))
    (:`3`
      (`SceneComponent.SetVisibility` (`self.Door3`) true false)))
  (return))

(fn `UserConstructionScript`
  (`self.Set Visibility` (`self.DoorAttribute`))
  (`parent.UserConstructionScript`))