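; Game instance Blueprint that serves per-level puzzle data and checks door answers, apparently for a molecule transport game.
; It builds the current level's molecule map from one of two level presets and looks up package spawn locations by stage.
; ValidateAnswer fetches expected answers by level and stage, requires equal counts, then matches doors regardless of order on passage type, side and specs.
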(fn `Answers Contains`
  (params (Answers :type "Array of /Game/Blueprints/S_ShallowOrder Structure") (Order :type "/Game/Blueprints/S_ShallowOrder Structure"))
  (returns (Contains :type Boolean))
  (locals (`Found Order` :type Boolean :default true))
  (bind (_passagetype _specs _onfromside) (break `/Game/Blueprints/S_ShallowOrder` Order))
  (for _array_element Answers
    (bind (_passagetype_2 _specs_2 _onfromside_2) (break `/Game/Blueprints/S_ShallowOrder` _array_element))
    (bind _output_get (set `local.Found Order` (and (== _passagetype_2 _passagetype) (== _onfromside_2 _onfromside) (== (`KismetArrayLibrary.Array_Length` _specs_2) (`KismetArrayLibrary.Array_Length` _specs)))))
    (if _output_get
      (for _array_element_2 _specs_2
        (if (not (`KismetArrayLibrary.Array_Contains` _specs _array_element_2))
          (set `local.Found Order` false)
          (break)))
      (if (`local.Found Order`)
        (break))))
  (return (`local.Found Order`)))

(fn `Get Molecules`
  (returns (`Molecule Map` :type "Map of String to /Game/Blueprints/S_Molecule Structure"))
  (locals (Result :type "Map of String to /Game/Blueprints/S_Molecule Structure") (`Level 1 Preset` :type "Array of String") (`Level 2 Preset` :type "Array of String"))
  (for _array_element (select `int` (`self.Current Level`) :`0` (`local.Level 1 Preset`) :`1` (`local.Level 2 Preset`))
    (bind (_value _returnvalue) (`BlueprintMapLibrary.Map_Find` (`self.Molecules`) _array_element))
    (if _returnvalue
      (`BlueprintMapLibrary.Map_Add` (`local.Result`) _array_element _value)))
  (return (`local.Result`)))

(fn `Get Package Spawn`
  (params (`Current Stage` :type Integer))
  (returns (Spawn :type "Vector Structure"))
  (locals (Locations :type "Array of Vector Structure"))
  (return (`|GetArrayItem` (`local.Locations`) `Current Stage`)))

(fn `Validate Answer`
  (params (Doors :type "Array of /Game/Blueprints/S_ShallowOrder Structure"))
  (returns (Correct :type Boolean))
  (locals (`Stage Answers` :type "Map of /Game/Blueprints/S_LevelStage Structure to /Game/Blueprints/S_Answers Structure") (`Has All` :type Boolean :default true))
  (bind _answers (break `/Game/Blueprints/S_Answers` (`BlueprintMapLibrary.Map_Find` (`local.Stage Answers`) (make `/Game/Blueprints/S_LevelStage` (`self.Current Level`) (`self.Current Stage`)))))
  (if (== (`KismetArrayLibrary.Array_Length` Doors) (`KismetArrayLibrary.Array_Length` _answers))
    (for _array_element _answers
      (if (not (`self.Answers Contains` Doors _array_element))
        (set `local.Has All` false)
        (break)))
    (return (`local.Has All`))
    (else
      (return false))))