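; BP_Interactable is a base interactable actor with an Interact function that returns false by default.
; Its construction script stores the first mesh found among the root's children in HighlightMeshes.
; SetActive calls SetHighlight, which toggles custom depth on those meshes for highlighting.
; Activation also shows a button prompt widget for actors tagged BP_Terminal, and deactivation removes it.
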(fn `Interact`
  (params (Interactor :type "Actor Object Reference"))
  (returns (Success :type Boolean))
  (return false))

(fn `Set Active`
  (params (Active :type Boolean))
  (`self.Set Highlight` Active))

(fn `Set Highlight`
  (params (Active :type Boolean))
  (if Active
    (if (`self.ActorHasTag` "BP_Terminal")
      (bind _returnvalue (`|CreateWidget` "/Game/UI/Widgets/WG_ButtonPrompt.WG_ButtonPrompt_C" (`GameplayStatics.GetPlayerController` 0)))
      (set `self.WG_ButtonPrompt` _returnvalue)
      (`UserWidget.AddToViewport` _returnvalue 0))
    (else
      (`Widget.RemoveFromParent` (`self.WG_ButtonPrompt`))))
  (for _array_element (`self.Highlight Meshes`)
    (`PrimitiveComponent.SetRenderCustomDepth` _array_element Active)))

(fn `UserConstructionScript`
  (for _array_element (`SceneComponent.GetChildrenComponents` (`self.DefaultSceneRoot`) true)
    (bind _asmesh_component (cast `MeshComponent` _array_element))
    (`KismetArrayLibrary.Array_Set` (`self.Highlight Meshes`) 0 _asmesh_component true)
    (break)))