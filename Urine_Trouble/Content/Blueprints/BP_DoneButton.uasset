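; BP_DoneButton is an interactable button that submits the player's answer to the game mode.
; Its Interact function casts the current game mode to UT_GameMode_BP, calls SubmitAnswer, then prints the result to screen and returns it.
; The event graph holds only disabled default stubs, so all behavior runs through Interact.
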(fn `Interact`
  (params (Interactor :type "Actor Object Reference"))
  (returns (Success :type Boolean))
  (bind _asut_game_mode_bp (cast `/Game/Blueprints/UT_GameMode_BP` (`GameplayStatics.GetGameMode`)))
  (bind _correct (`/Game/Blueprints/UT_GameMode_BP.Submit Answer` _asut_game_mode_bp))
  (`KismetSystemLibrary.PrintString` (`KismetStringLibrary.Conv_BoolToString` _correct))
  (return _correct))

(fn `UserConstructionScript`
  (`parent.UserConstructionScript`))