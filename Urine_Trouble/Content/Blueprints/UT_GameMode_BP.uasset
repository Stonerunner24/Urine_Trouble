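; Game mode for a molecule passage puzzle that handles ordering passages as deliveries and checking the player's answer.
; On BeginPlay it spawns an unbound post-process volume with a highlight material and reads molecules and package spawn from the game instance.
; OrderPassage spawns a delivery at that point carrying door info and a shallow order built from the passage specs.
; SubmitAnswer gathers every doorway's order for the game instance to validate.
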(event `self.ReceiveBeginPlay`
  (`self.Make Highlight Volume`)
  (set `self.Passages Ordered` 0)
  (bind _asut_game_instance_bp (cast `/Game/Blueprints/UT_GameInstance_BP` (`GameplayStatics.GetGameInstance`)))
  (set `self.Molecules` (`/Game/Blueprints/UT_GameInstance_BP.Get Molecules` _asut_game_instance_bp))
  (set `self.Package Spawn` (`/Game/Blueprints/UT_GameInstance_BP.Get Package Spawn` _asut_game_instance_bp 0)))

(fn `Make Highlight Volume`
  (bind _returnvalue (`|SpawnActorFromClass` (`self.PPV_Ref`) (`KismetMathLibrary.MakeTransform` (0.0 0.0 0.0)) "Undefined" "MultiplyWithRoot" null null))
  (set `PostProcessVolume.bUnbound` true _returnvalue)
  (setmembers `PostProcessSettings` :`StructRef` (`PostProcessVolume.Settings` _returnvalue) :`WeightedBlendables` (make `WeightedBlendables` (`|MakeArray` (make `WeightedBlendable` 1.0 "/Game/Materials/HighlightMat.HighlightMat")))))

(fn `Order Passage`
  (params (Passage :type "/Game/Blueprints/S_Order Structure"))
  (locals (Specs :type "Array of /Game/Blueprints/S_ShallowSpec Structure"))
  (bind (_passagetype _specs) (break `/Game/Blueprints/S_Order` Passage))
  (`/Engine/EditorBlueprintResources/StandardMacros.IncrementInt` (`self.Passages Ordered`)
    (:`  `
      (bind _returnvalue (`|SpawnActorFromClass` "/Game/Blueprints/BP_Delivery.BP_Delivery_C" (`KismetMathLibrary.MakeTransform` (`self.Package Spawn`)) "Undefined" "MultiplyWithRoot" null null))
      (bind _structout (setmembers `/Game/Blueprints/StructDoor_BP` :`StructRef` (make `/Game/Blueprints/StructDoor_BP` _passagetype _specs)))
      (set `/Game/Blueprints/BP_Delivery.DoorInfo` _structout _returnvalue)
      (for _array_element _specs
        (bind (_molecule _flowdirection _moleculeqty) (break `/Game/Blueprints/S_MoleculeSpec` _array_element))
        (`KismetArrayLibrary.Array_Add` (`local.Specs`) (make `/Game/Blueprints/S_ShallowSpec` (`KismetTextLibrary.Conv_TextToString` (break `/Game/Blueprints/S_Molecule` _molecule)) _flowdirection _moleculeqty)))
      (set `/Game/Blueprints/BP_Delivery.Door Order` (make `/Game/Blueprints/S_ShallowOrder` _passagetype (`local.Specs`)) _returnvalue))))

(fn `Submit Answer`
  (returns (Correct :type Boolean))
  (locals (Guesses :type "Array of /Game/Blueprints/S_ShallowOrder Structure"))
  (bind _guesses (`local.Guesses`))
  (bind _asut_game_instance_bp (cast `/Game/Blueprints/UT_GameInstance_BP` (`GameplayStatics.GetGameInstance`))
    (:`then`
      (bind _outactors (`GameplayStatics.GetAllActorsOfClass` "/Game/Blueprints/BP_Doorway.BP_Doorway_C"))
      (for _array_element _outactors
        (bind _door_order (`/Game/Blueprints/BP_Doorway.Door Order` _array_element))
        (`KismetArrayLibrary.Array_Add` _guesses _door_order)
        (`KismetSystemLibrary.PrintString` (`KismetStringLibrary.Conv_IntToString` (`.PassageType_2_11C3400641ED59685039A2B25BCA73D5` (break `/Game/Blueprints/S_ShallowOrder` _door_order)))))
      (bind _correct (`/Game/Blueprints/UT_GameInstance_BP.Validate Answer` _asut_game_instance_bp _guesses))
      (return _correct))
    (:`CastFailed`
      (return false))))

(fn `UserConstructionScript`)