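; BP_Terminal is an interactable terminal that guides BP_Renaldo into position to use its screen widget.
; It creates a WG_Terminal widget once at BeginPlay.
; Interact passes that widget to Renaldo's OnBeginGuide, using the GuidePosition arrow's tip as the destination and its origin as the look target.
; It then plays a boot sound and returns true; any other interactor gets false.
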(event `self.ReceiveBeginPlay`
  (bind _returnvalue (`|CreateWidget` "/Game/UI/Widgets/WG_Terminal.WG_Terminal_C"))
  (set `self.Widget` _returnvalue))

(fn `Interact`
  (params (Interactor :type "Actor Object Reference"))
  (returns (Success :type Boolean))
  (bind _guide_position (`self.Guide Position`))
  (bind _returnvalue (`SceneComponent.K2_GetComponentLocation` _guide_position))
  (bind _asbp_renaldo (cast `/Game/Blueprints/BP_Renaldo` Interactor)
    (:`then`
      (`/Game/Blueprints/BP_Renaldo.On Begin Guide` _asbp_renaldo (+ _returnvalue (* (`SceneComponent.GetForwardVector` _guide_position) (`ArrowComponent.ArrowLength` _guide_position))) _returnvalue 0.25 (`self.Widget`))
      (`GameplayStatics.PlaySound2D` "/Game/Audio/SoundFX/Terminal_Boot.Terminal_Boot" 0.5 1.0 0.0 null null)
      (return true))
    (:`CastFailed`
      (return false))))

(fn `UserConstructionScript`)