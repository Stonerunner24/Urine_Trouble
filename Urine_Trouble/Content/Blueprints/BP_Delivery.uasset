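; BP_Delivery is an interactable delivery pickup that hands door data to the player character, BP_Renaldo.
; On BeginPlay it plays a 2D box-drop sound.
; Interact casts player pawn 0 to BP_Renaldo rather than using the Interactor argument, copies DoorInfo and DoorOrder onto it, then destroys itself and returns true.
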(event `self.ReceiveBeginPlay`
  (`parent.ReceiveBeginPlay`)
  (`GameplayStatics.PlaySound2D` "/Game/Audio/SoundFX/Door_BoxDrop.Door_BoxDrop" 1.0 1.0 0.0 null null))

(fn `Interact`
  (params (Interactor :type "Actor Object Reference"))
  (returns (Success :type Boolean))
  (bind _asbp_renaldo (cast `/Game/Blueprints/BP_Renaldo` (`GameplayStatics.GetPlayerPawn` 0)))
  (set `/Game/Blueprints/BP_Renaldo.Door` (`self.DoorInfo`) _asbp_renaldo)
  (set `/Game/Blueprints/BP_Renaldo.Door Order` (`self.Door Order`) _asbp_renaldo)
  (`self.K2_DestroyActor`)
  (return true))

(fn `UserConstructionScript`
  (`parent.UserConstructionScript`))